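; Table actor that scatters plates over its surface and acts as the plate washer.
; On BeginPlay or checkSpawn, it spawns as many Bp_plate actors as the VR pawn's PlatesNumber.
; RandomLocation picks points in SpawnArea's bounds, retrying when a radial distance test against NotSpawnArea flags the sink.
; Plates that begin overlapping the DishWash component get Poped called on them.
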(event `self.ReceiveBeginPlay`
  ;[0.8971 1 0.05759] Spawn plates on Table
  (bind _asmy_vrpawn (cast `/Game/Assets/player/myVRPawn` (`GameplayStatics.GetPlayerPawn` 0) :!label _label))
  (for _ (range (+ (`/Game/Assets/player/myVRPawn.platesNumber` _asmy_vrpawn) 1))
    (bind (_notoversink _spawnlocation) (`self.randomLocation` :!label _label_2))
    (if _notoversink
      (`|SpawnActorFromClass` "/Game/Assets/blueprints/bp_plate.bp_plate_C" (`KismetMathLibrary.MakeTransform` _spawnlocation) "Undefined" "OverrideRootScale")
      (else
        (goto _label_2)))))

(event `checkSpawn`
  ;[0.8971 1 0.05759] Spawn plates on Table
  (goto _label))

(event `self.dishWash.OnComponentBeginOverlap`
  (params (OverlappedComponent :type "PrimitiveComponent Object Reference") (OtherActor :type "Actor Object Reference") (OtherComp :type "PrimitiveComponent Object Reference") (OtherBodyIndex :type Integer) (bFromSweep :type Boolean) (SweepResult :type "HitResult Structure (by ref)"))
  ;[1 0.1516 0.02183] Plate washer
  (if (== (`GameplayStatics.GetObjectClass` OtherActor) "/Game/Assets/blueprints/bp_plate.bp_plate_C")
    (bind _asbp_plate (cast `/Game/Assets/blueprints/bp_plate` OtherActor))
    (`/Game/Assets/blueprints/bp_plate.poped` _asbp_plate)))

(fn `randomLocation`
  (returns (notOverSink :type Boolean) (spawnLocation :type "Vector Structure"))
  (bind (_origin _boxextent) (`KismetSystemLibrary.GetComponentBounds` (`self.notSpawnArea`)))
  (bind (_origin_2 _boxextent_2) (`KismetSystemLibrary.GetComponentBounds` (`self.spawnArea`)))
  (bind _returnvalue (`KismetMathLibrary.RandomPointInBoundingBox` _origin_2 _boxextent_2))
  (return (> (`KismetMathLibrary.VSize` (- _origin _returnvalue)) (+ (.x _boxextent) 3.0)) _returnvalue))

(fn `UserConstructionScript`)