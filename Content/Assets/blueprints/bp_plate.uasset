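; Plate actor that can be picked up, dropped and popped into confetti.
; On BeginPlay it binds to the pop-plates event of the first Bp_spawnTable found, which triggers a short delay, a confetti burst at the mesh, then self-destruction.
; PickUp disables mesh physics and attaches the root to the given parent, while DropOff re-enables physics and detaches the mesh, keeping world transforms.
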(event `self.ReceiveBeginPlay`
  (bind _outactors (`GameplayStatics.GetAllActorsOfClass` "/Game/Assets/blueprints/bp_spawnTable.bp_spawnTable_C"))
  (add `/Game/Assets/blueprints/bp_spawnTable.popPlates` (`KismetArrayLibrary.Array_Get` _outactors) (delegate `poped`)))

(event `poped`
  (`KismetSystemLibrary.Delay` 1.5)
  (`GameplayStatics.SpawnEmitterAtLocation` "/Game/Assets/additionalresources/p_confetti.p_confetti" (`SceneComponent.K2_GetComponentLocation` (`self.plate_mesh`)))
  (`self.K2_DestroyActor`))

(event `/Game/Assets/blueprints/PickUpDropOffInterface.pickUp`
  (params (ActorToAttachTo :type "SceneComponent Object Reference"))
  (`PrimitiveComponent.SetSimulatePhysics` (`self.plate_mesh`) false)
  (`SceneComponent.K2_AttachToComponent` (`self.K2_GetRootComponent`) ActorToAttachTo "None" "KeepWorld" "KeepWorld" "KeepWorld" false))

(event `/Game/Assets/blueprints/PickUpDropOffInterface.dropOff`
  (bind _plate_mesh (`self.plate_mesh`))
  (`PrimitiveComponent.SetSimulatePhysics` _plate_mesh true)
  (`SceneComponent.K2_DetachFromComponent` _plate_mesh "KeepWorld" "KeepWorld" "KeepWorld" false))

(fn `UserConstructionScript`)